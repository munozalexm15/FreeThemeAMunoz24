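; Camera actor for the badminton game that can turn to follow the shuttlecock, controlled by a player setting.
; On BeginPlay it finds and caches the Shuttlecock_Blueprint actor.
; Each tick, if the CameraFollowsShuttlecock option in the game mode's settings save is on, it eases the camera component's rotation toward the shuttlecock sprite using FindLookAtRotation and RInterpTo.
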(event EventBeginPlay
  (bind _returnvalue (Actor|GetActorOfClass "/Game/Blueprints/Shuttlecock/Shuttlecock_Blueprint.Shuttlecock_Blueprint_C"))
  (Variables|Default|SetShuttlecock _returnvalue))

(event Collision|EventActorBeginOverlap
  (params (OtherActor :type Actor%20Object%20Reference)))

(event EventTick
  (params (DeltaSeconds :type Float%20%28single-precision%29))
  ;[1 1 1] Update camera rotation to look at shuttlecock (Lerp)
  (bind _asgoodminton_game_mode (Utilities|Casting|CastToGoodminton_GameMode (Game|GetGameMode)))
  (bind _assettings_save_game (Utilities|Casting|CastToSettings_SaveGame (Variables|/Game/GameMode/Goodminton_GameMode.Goodminton_GameMode_C|GetConfigSettings _asgoodminton_game_mode)))
  (if (Variables|/Game/SaveGames/Settings_SaveGame.Settings_SaveGame_C|GetCameraFollowsShuttlecock _assettings_save_game)
    (Transformation|SetWorldRotation (Variables|CameraActor|GetCameraComponent) (Math|Interpolation|RInterpTo (Transformation|GetWorldRotation (Variables|CameraActor|GetCameraComponent)) (Math|Rotator|FindLookatRotation (Transformation|GetWorldLocation (Variables|CameraActor|GetCameraComponent)) (Transformation|GetWorldLocation (Variables|/Game/Blueprints/Shuttlecock/Shuttlecock_Blueprint.Shuttlecock_Blueprint_C|GetPaperSprite (Variables|Default|GetShuttlecock)))) (/ (Utilities|Time|GetWorldDeltaSeconds) 2.0) 2.0) false false)))

(fn ConstructionScript)