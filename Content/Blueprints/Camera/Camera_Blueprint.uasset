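; Camera actor that keeps its Camera component aimed at the shuttlecock as it moves.
; BeginPlay caches player 0's TraceurCharacter_PlayerControllerBP and, only if that cast succeeds, finds the Shuttlecock_Blueprint actor in the level.
; Every Tick sets the camera's world rotation with a look-at toward the shuttlecock, with no smoothing or validity check.
; The stored controller reference is not used elsewhere in this Blueprint.
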(event EventBeginPlay
  (bind _astraceur_character_player_controller_bp (Utilities|Casting|CastToTraceurCharacter_PlayerControllerBP (Game|GetPlayerController 0)))
  (Variables|Default|SetCharacter%20Player%20BP _astraceur_character_player_controller_bp)
  (bind _returnvalue (Actor|GetActorOfClass "/Game/Blueprints/Shuttlecock/Shuttlecock_Blueprint.Shuttlecock_Blueprint_C"))
  (Variables|Default|SetShuttlecock _returnvalue))

(event Collision|EventActorBeginOverlap
  (params (OtherActor :type Actor%20Object%20Reference)))

(event EventTick
  (params (DeltaSeconds :type Float%20%28single-precision%29))
  (Transformation|SetWorldRotation (Variables|Default|GetCamera) (Math|Rotator|FindLookatRotation (Transformation|GetWorldLocation (Variables|Default|GetCamera)) (Transformation|GetActorLocation (Variables|Default|GetShuttlecock))) false false))

(fn ConstructionScript)