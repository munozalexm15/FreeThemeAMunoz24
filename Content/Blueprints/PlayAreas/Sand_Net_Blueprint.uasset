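; Sand net play area that scores Goodminton rallies from shuttlecock overlaps with its trigger components.
; Field hits add a point to the same-named side, give serve to the last hitter, restart the round and re-allow movement after a delay.
; End areas only score for the opposite side, except LeftSideDownEndArea, whose increment is disconnected.
; FieldGround restarts the round without scoring, and all scores live in Goodminton_GameMode.
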(event OnComponentBeginOverlap(LeftAreaEndArea)
  (params (OverlappedComponent :type Primitive%20Component%20Object%20Reference) (OtherActor :type Actor%20Object%20Reference) (OtherComp :type Primitive%20Component%20Object%20Reference) (OtherBodyIndex :type Integer) (bFromSweep :type Boolean) (SweepResult :type Hit%20Result%20Structure%20%28by%20ref%29))
  ;[1 1 1] Give point to right
  (bind _asshuttlecock_blueprint (Utilities|Casting|CastToShuttlecock_Blueprint OtherActor))
  (if (== (Variables|/Game/Blueprints/Shuttlecock/Shuttlecock_Blueprint.Shuttlecock_Blueprint_C|GetPhysic _asshuttlecock_blueprint) OtherComp)
    (bind _asgoodminton_game_mode (Utilities|Casting|CastToGoodminton_GameMode (Game|GetGameMode)))
    (Variables|/Game/GameMode/Goodminton_GameMode.Goodminton_GameMode_C|SetRightPoints _asgoodminton_game_mode (+ (Variables|/Game/GameMode/Goodminton_GameMode.Goodminton_GameMode_C|GetRightPoints _asgoodminton_game_mode) 1))))

(event OnComponentBeginOverlap(playArea_Field_Plane_008)
  (params (OverlappedComponent :type Primitive%20Component%20Object%20Reference) (OtherActor :type Actor%20Object%20Reference) (OtherComp :type Primitive%20Component%20Object%20Reference) (OtherBodyIndex :type Integer) (bFromSweep :type Boolean) (SweepResult :type Hit%20Result%20Structure%20%28by%20ref%29)))

(event OnComponentBeginOverlap(FieldGround)
  (params (OverlappedComponent :type Primitive%20Component%20Object%20Reference) (OtherActor :type Actor%20Object%20Reference) (OtherComp :type Primitive%20Component%20Object%20Reference) (OtherBodyIndex :type Integer) (bFromSweep :type Boolean) (SweepResult :type Hit%20Result%20Structure%20%28by%20ref%29))
  ;[1 1 1] If it is out of bounds
  (bind _asshuttlecock_blueprint (Utilities|Casting|CastToShuttlecock_Blueprint OtherActor))
  (if (== (Variables|/Game/Blueprints/Shuttlecock/Shuttlecock_Blueprint.Shuttlecock_Blueprint_C|GetPhysic _asshuttlecock_blueprint) OtherComp)
    (bind _asgoodminton_game_mode (Utilities|Casting|CastToGoodminton_GameMode (Game|GetGameMode)))
    (Default|StartRound _asgoodminton_game_mode)))

(event OnComponentBeginOverlap(AreaDelimiter)
  (params (OverlappedComponent :type Primitive%20Component%20Object%20Reference) (OtherActor :type Actor%20Object%20Reference) (OtherComp :type Primitive%20Component%20Object%20Reference) (OtherBodyIndex :type Integer) (bFromSweep :type Boolean) (SweepResult :type Hit%20Result%20Structure%20%28by%20ref%29)))

(event OnComponentBeginOverlap(RightAreaEndArea)
  (params (OverlappedComponent :type Primitive%20Component%20Object%20Reference) (OtherActor :type Actor%20Object%20Reference) (OtherComp :type Primitive%20Component%20Object%20Reference) (OtherBodyIndex :type Integer) (bFromSweep :type Boolean) (SweepResult :type Hit%20Result%20Structure%20%28by%20ref%29))
  (bind _asshuttlecock_blueprint (Utilities|Casting|CastToShuttlecock_Blueprint OtherActor))
  (if (== (Variables|/Game/Blueprints/Shuttlecock/Shuttlecock_Blueprint.Shuttlecock_Blueprint_C|GetPhysic _asshuttlecock_blueprint) OtherComp)
    (bind _asgoodminton_game_mode (Utilities|Casting|CastToGoodminton_GameMode (Game|GetGameMode)))
    (Variables|/Game/GameMode/Goodminton_GameMode.Goodminton_GameMode_C|SetLeftPoints _asgoodminton_game_mode (+ (Variables|/Game/GameMode/Goodminton_GameMode.Goodminton_GameMode_C|GetLeftPoints _asgoodminton_game_mode) 1))))

(event OnComponentBeginOverlap(LeftSideDownEndArea)
  (params (OverlappedComponent :type Primitive%20Component%20Object%20Reference) (OtherActor :type Actor%20Object%20Reference) (OtherComp :type Primitive%20Component%20Object%20Reference) (OtherBodyIndex :type Integer) (bFromSweep :type Boolean) (SweepResult :type Hit%20Result%20Structure%20%28by%20ref%29))
  ;[1 1 1] Give point to right
  (bind _asshuttlecock_blueprint (Utilities|Casting|CastToShuttlecock_Blueprint OtherActor))
  (if (== (Variables|/Game/Blueprints/Shuttlecock/Shuttlecock_Blueprint.Shuttlecock_Blueprint_C|GetPhysic _asshuttlecock_blueprint) OtherComp)
    (bind _asgoodminton_game_mode (Utilities|Casting|CastToGoodminton_GameMode (Game|GetGameMode)))))

(event OnComponentBeginOverlap(RightSideUpEndArea)
  (params (OverlappedComponent :type Primitive%20Component%20Object%20Reference) (OtherActor :type Actor%20Object%20Reference) (OtherComp :type Primitive%20Component%20Object%20Reference) (OtherBodyIndex :type Integer) (bFromSweep :type Boolean) (SweepResult :type Hit%20Result%20Structure%20%28by%20ref%29))
  (bind _asshuttlecock_blueprint (Utilities|Casting|CastToShuttlecock_Blueprint OtherActor))
  (if (== (Variables|/Game/Blueprints/Shuttlecock/Shuttlecock_Blueprint.Shuttlecock_Blueprint_C|GetPhysic _asshuttlecock_blueprint) OtherComp)
    (bind _asgoodminton_game_mode (Utilities|Casting|CastToGoodminton_GameMode (Game|GetGameMode)))
    (Variables|/Game/GameMode/Goodminton_GameMode.Goodminton_GameMode_C|SetLeftPoints _asgoodminton_game_mode (+ (Variables|/Game/GameMode/Goodminton_GameMode.Goodminton_GameMode_C|GetLeftPoints _asgoodminton_game_mode) 1))))

(event OnComponentBeginOverlap(LeftSideUpEndArea)
  (params (OverlappedComponent :type Primitive%20Component%20Object%20Reference) (OtherActor :type Actor%20Object%20Reference) (OtherComp :type Primitive%20Component%20Object%20Reference) (OtherBodyIndex :type Integer) (bFromSweep :type Boolean) (SweepResult :type Hit%20Result%20Structure%20%28by%20ref%29))
  ;[1 1 1] Give point to right
  (bind _asshuttlecock_blueprint (Utilities|Casting|CastToShuttlecock_Blueprint OtherActor))
  (if (== (Variables|/Game/Blueprints/Shuttlecock/Shuttlecock_Blueprint.Shuttlecock_Blueprint_C|GetPhysic _asshuttlecock_blueprint) OtherComp)
    (bind _asgoodminton_game_mode (Utilities|Casting|CastToGoodminton_GameMode (Game|GetGameMode)))
    (Variables|/Game/GameMode/Goodminton_GameMode.Goodminton_GameMode_C|SetRightPoints _asgoodminton_game_mode (+ (Variables|/Game/GameMode/Goodminton_GameMode.Goodminton_GameMode_C|GetRightPoints _asgoodminton_game_mode) 1))))

(event OnComponentBeginOverlap(RightSideDownEndArea)
  (params (OverlappedComponent :type Primitive%20Component%20Object%20Reference) (OtherActor :type Actor%20Object%20Reference) (OtherComp :type Primitive%20Component%20Object%20Reference) (OtherBodyIndex :type Integer) (bFromSweep :type Boolean) (SweepResult :type Hit%20Result%20Structure%20%28by%20ref%29))
  (bind _asshuttlecock_blueprint (Utilities|Casting|CastToShuttlecock_Blueprint OtherActor))
  (if (== (Variables|/Game/Blueprints/Shuttlecock/Shuttlecock_Blueprint.Shuttlecock_Blueprint_C|GetPhysic _asshuttlecock_blueprint) OtherComp)
    (bind _asgoodminton_game_mode (Utilities|Casting|CastToGoodminton_GameMode (Game|GetGameMode)))
    (Variables|/Game/GameMode/Goodminton_GameMode.Goodminton_GameMode_C|SetLeftPoints _asgoodminton_game_mode (+ (Variables|/Game/GameMode/Goodminton_GameMode.Goodminton_GameMode_C|GetLeftPoints _asgoodminton_game_mode) 1))))

(event OnComponentBeginOverlap(RightField)
  (params (OverlappedComponent :type Primitive%20Component%20Object%20Reference) (OtherActor :type Actor%20Object%20Reference) (OtherComp :type Primitive%20Component%20Object%20Reference) (OtherBodyIndex :type Integer) (bFromSweep :type Boolean) (SweepResult :type Hit%20Result%20Structure%20%28by%20ref%29))
  ;[1 1 1] Point for right field, left field begins turn
  (bind _asshuttlecock_blueprint (Utilities|Casting|CastToShuttlecock_Blueprint OtherActor))
  (if (== (Variables|/Game/Blueprints/Shuttlecock/Shuttlecock_Blueprint.Shuttlecock_Blueprint_C|GetPhysic _asshuttlecock_blueprint) OtherComp)
    ;[1 1 1] Set who is going to serve (ATM, the one who points is going to serve)
    (bind _asgoodminton_game_mode (Utilities|Casting|CastToGoodminton_GameMode (Game|GetGameMode)))
    (Variables|/Game/GameMode/Goodminton_GameMode.Goodminton_GameMode_C|SetRightPoints _asgoodminton_game_mode (+ (Variables|/Game/GameMode/Goodminton_GameMode.Goodminton_GameMode_C|GetRightPoints _asgoodminton_game_mode) 1))
    (Variables|/Game/GameMode/Goodminton_GameMode.Goodminton_GameMode_C|SetPlayerServe _asgoodminton_game_mode (Variables|/Game/Blueprints/Shuttlecock/Shuttlecock_Blueprint.Shuttlecock_Blueprint_C|GetLastHitCharacter _asshuttlecock_blueprint))
    (Default|StartRound _asgoodminton_game_mode)
    (Utilities|FlowControl|Delay 2.0)
    (Default|AllowMovement _asgoodminton_game_mode)))

(event OnComponentBeginOverlap(LeftField)
  (params (OverlappedComponent :type Primitive%20Component%20Object%20Reference) (OtherActor :type Actor%20Object%20Reference) (OtherComp :type Primitive%20Component%20Object%20Reference) (OtherBodyIndex :type Integer) (bFromSweep :type Boolean) (SweepResult :type Hit%20Result%20Structure%20%28by%20ref%29))
  (bind _asshuttlecock_blueprint (Utilities|Casting|CastToShuttlecock_Blueprint OtherActor))
  (if (== (Variables|/Game/Blueprints/Shuttlecock/Shuttlecock_Blueprint.Shuttlecock_Blueprint_C|GetPhysic _asshuttlecock_blueprint) OtherComp)
    ;[1 1 1] Set who is going to serve (ATM, the one who points is going to serve)
    (bind _asgoodminton_game_mode (Utilities|Casting|CastToGoodminton_GameMode (Game|GetGameMode)))
    (Variables|/Game/GameMode/Goodminton_GameMode.Goodminton_GameMode_C|SetLeftPoints _asgoodminton_game_mode (+ (Variables|/Game/GameMode/Goodminton_GameMode.Goodminton_GameMode_C|GetLeftPoints _asgoodminton_game_mode) 1))
    (Variables|/Game/GameMode/Goodminton_GameMode.Goodminton_GameMode_C|SetPlayerServe _asgoodminton_game_mode (Variables|/Game/Blueprints/Shuttlecock/Shuttlecock_Blueprint.Shuttlecock_Blueprint_C|GetLastHitCharacter _asshuttlecock_blueprint))
    (Default|StartRound _asgoodminton_game_mode)
    (Utilities|FlowControl|Delay 2.0)
    (Default|AllowMovement _asgoodminton_game_mode)))

(event EventBeginPlay)

(event Collision|EventActorBeginOverlap
  (params (OtherActor :type Actor%20Object%20Reference)))

(event EventTick
  (params (DeltaSeconds :type Float%20%28single-precision%29)))

(fn ConstructionScript)