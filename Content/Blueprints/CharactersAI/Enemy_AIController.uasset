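; AI controller for an enemy that tracks and hits a shuttlecock.
; On BeginPlay it runs NormalIA_BehaviorTree, writes HitRange to the Blackboard, caches the Shuttlecock actor and draws a debug sphere around its pawn.
; Sight perception updates set the IsInField and CanHit Blackboard keys.
; CanHit compares the squared pawn-to-shuttlecock distance against the unsquared HitRANGE, and refreshes only on those updates.
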(event OnTargetPerceptionUpdated(AIPerception)
  (params (Actor :type Actor%20Object%20Reference) (Stimulus :type AI%20Stimulus%20Structure))
  (bind _returnvalue (Class|AIPerceptionSystem|GetSenseClassforStimulus Stimulus))
  (if (== _returnvalue "/Script/AIModule.AISense_Sight")
    (AI|Components|Blackboard|SetValueasBool (AI|GetBlackboard 0) (Utilities|Name|MakeLiteralName "IsInField") (.bSuccessfullySensed (Utilities|Struct|BreakAIStimulus Stimulus)))
    (AI|Components|Blackboard|SetValueasBool (AI|GetBlackboard 0) (Utilities|Name|MakeLiteralName "CanHit") (< (Class|KismetMathLibrary|VectorDistanceSquared (Transformation|GetActorLocation (Variables|Default|GetShuttlecock)) (Transformation|GetActorLocation (Pawn|GetControlledPawn))) (Variables|Default|GetHitRANGE)))))

(event EventBeginPlay
  (AI|RunBehaviorTree "/Game/Blueprints/CharactersAI/NormalIA_BehaviorTree.NormalIA_BehaviorTree")
  (AI|Components|Blackboard|SetValueasFloat (AI|GetBlackboard 0) (Utilities|Name|MakeLiteralName "HitRange") (Variables|Default|GetHitRANGE))
  (bind _returnvalue (Actor|GetActorOfClass "/Game/Blueprints/Shuttlecock/Shuttlecock_Blueprint.Shuttlecock_Blueprint_C"))
  (Variables|Default|SetShuttlecock _returnvalue)
  (Rendering|Debug|DrawDebugSphere (Transformation|GetActorLocation (Pawn|GetControlledPawn)) 3.5e+02 12 "(R=1.000000,G=1.000000,B=1.000000,A=1.000000)" 1e+02 2.0))

(event EventTick
  (params (DeltaSeconds :type Float%20%28single-precision%29)))

(fn ConstructionScript)