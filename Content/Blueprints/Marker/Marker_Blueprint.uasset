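; Marker actor that acts as a ground indicator beneath the shuttlecock, showing its position over the court.
; On BeginPlay it sets a half-transparent white tint and caches the shuttlecock and net actors, the latter serving as the field reference.
; Each tick it follows the shuttlecock's X/Y at a fixed Z and fades linearly as the shuttlecock rises above the play-area plane.
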(event EventBeginPlay
  (Utilities|FlowControl|Sequence
    (:then_0
      (Sprite|SetSpriteColor (Variables|Default|GetMarker) (Utilities|Struct|MakeLinearColor 1.0 1.0 1.0 0.5)))
    (:then_1
      (bind _returnvalue (Actor|GetActorOfClass "/Game/Blueprints/Shuttlecock/Shuttlecock_Blueprint.Shuttlecock_Blueprint_C"))
      (Variables|Default|SetShuttlecock _returnvalue)
      (bind _returnvalue_2 (Actor|GetActorOfClass "/Game/Blueprints/PlayAreas/Net_Blueprint.Net_Blueprint_C"))
      (Variables|Default|SetField _returnvalue_2))))

(event Collision|EventActorBeginOverlap
  (params (OtherActor :type Actor%20Object%20Reference)))

(event EventTick
  (params (DeltaSeconds :type Float%20%28single-precision%29))
  (bind _shuttlecock (Variables|Default|GetShuttlecock))
  (bind _papersprite (Variables|/Game/Blueprints/Shuttlecock/Shuttlecock_Blueprint.Shuttlecock_Blueprint_C|GetPaperSprite _shuttlecock))
  (bind _returnvalue (Transformation|GetWorldLocation _papersprite))
  (Transformation|SetWorldLocation (Variables|Default|GetMarker) (Math|Vector|MakeVector (.x _returnvalue) (.y _returnvalue) 1.0) false false)
  (bind _output_get (Variables|Default|SetOpacity (- (Variables|Default|GetOpacity) (/ (- (.z (Transformation|GetWorldLocation (Variables|/Game/Blueprints/Shuttlecock/Shuttlecock_Blueprint.Shuttlecock_Blueprint_C|GetPaperSprite (Variables|Default|GetShuttlecock)))) (.z (Transformation|GetWorldLocation (Variables|/Game/Blueprints/PlayAreas/Net_Blueprint.Net_Blueprint_C|GetplayArea_Field_Plane (Variables|Default|GetField))))) 2e+02))))
  (Sprite|SetSpriteColor (Variables|Default|GetMarker) (Utilities|Struct|MakeLinearColor 1.0 1.0 1.0 _output_get))
  (Variables|Default|SetOpacity 1.0))

(fn ConstructionScript)